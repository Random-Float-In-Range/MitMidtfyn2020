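; Asteroid actor that drifts and spins with randomized motion.
; The construction script sets a random roll and picks a random drift velocity in the local YZ plane and a random roll spin rate.
; BeginPlay passes these to the RotatingMovement and ProjectileMovement components, applying the velocity in local space.
; Random actor scaling and box rescaling nodes are disconnected and never run.
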(event `self.ReceiveBeginPlay`
  (set `RotatingMovementComponent.RotationRate` (`self.Rotation`) (`self.RotatingMovement`))
  (`ProjectileMovementComponent.SetVelocityInLocalSpace` (`self.ProjectileMovement`) (`self.Direction`)))

(fn `UserConstructionScript`
  (`self.K2_SetActorRelativeRotation` (`KismetMathLibrary.MakeRotator` (`KismetMathLibrary.RandomFloatInRange` -90.0 90.0)))
  (set `self.Direction` (`KismetMathLibrary.MakeVector` 0.0 (`KismetMathLibrary.RandomFloatInRange` -60.0 60.0) (`KismetMathLibrary.RandomFloatInRange` -60.0 60.0)))
  (set `self.Rotation` (`KismetMathLibrary.MakeRotator` (`KismetMathLibrary.RandomFloatInRange` -30.0 30.0))))