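; Trampoline actor that bounces any Character overlapping it along the trampoline's up vector.
; Each axis of the launch scales that up vector by the character's absolute velocity on that axis times Elasticity, plus AdditionalForce.
; The launch adds to existing velocity rather than overriding it, and a jump sound plays at the character's location with attenuation.
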(event `self.ReceiveActorBeginOverlap`
  (params (OtherActor :type "Actor Object Reference"))
  (bind (_returnvalue_x _returnvalue_y _returnvalue_z) (`KismetMathLibrary.BreakVector` (`self.GetVelocity` OtherActor)))
  (bind _elasticity (`self.Elasticity`))
  (bind _additionalforce (`self.AdditionalForce`))
  (bind _ascharacter (cast `Character` OtherActor))
  (`Character.LaunchCharacter` _ascharacter (* (`KismetMathLibrary.GetUpVector` (`self.K2_GetActorRotation`)) (`KismetMathLibrary.MakeVector` (+ (* (`KismetMathLibrary.Abs` _returnvalue_x) _elasticity) _additionalforce) (+ (* (`KismetMathLibrary.Abs` _returnvalue_y) _elasticity) _additionalforce) (+ (* (`KismetMathLibrary.Abs` _returnvalue_z) _elasticity) _additionalforce))) false false)
  (`GameplayStatics.PlaySoundAtLocation` "/Game/JEMO/JEMO_ASSETS/Blueprints/350901__cabled-mess__jump-c-06_Cue.350901__cabled-mess__jump-c-06_Cue" (`self.K2_GetActorLocation` OtherActor) (struct) 1.0 1.0 0.0 "/Game/Mixed_FREE_Template_Assets/MilitaryWeapSilver/Sound/Attenuation/WeaponShot_att.WeaponShot_att" null null))

(fn `UserConstructionScript`)