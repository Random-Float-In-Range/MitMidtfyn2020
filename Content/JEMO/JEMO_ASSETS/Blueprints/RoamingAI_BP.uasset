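; Roaming AI character, apparently a cow, that wanders to random reachable points nearby and moos when something overlaps its sphere.
; Tick traces downward to align the body with the ground normal, then uses a random delay before each AIMoveTo.
; A DoOnce with a delayed reset throttles the moo, which fires for any overlapping actor.
; Projectile damage, death effects and the player-only overlap check are disconnected and never run.
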(event `self.ReceiveTick`
  (params (DeltaSeconds :type "Float (single-precision)"))
  (bind _returnvalue (`self.K2_GetActorLocation`))
  ;[1 1 1] Tick
  ;[1 1 1] Move to random location when player is out of sight
  ;;[1 1 1] LineTrace and project vector on ground, to make actor touch ground when moving.
  (bind (_outhit _returnvalue_2) (`KismetSystemLibrary.LineTraceSingle` _returnvalue (+ _returnvalue (* (`self.GetActorUpVector`) -200.0)) "TraceTypeQuery1" true))
  (if _returnvalue_2
    (bind (_bblockinghit _binitialoverlap _time _distance _location _impactpoint _normal) (`GameplayStatics.BreakHitResult` _outhit))
    (`self.K2_SetActorRotation` (`KismetMathLibrary.MakeRotFromXZ` (`KismetMathLibrary.ProjectVectorOnToPlane` (`self.GetActorForwardVector`) _normal) _normal))
    (`KismetSystemLibrary.Delay` (`KismetMathLibrary.RandomFloatInRange` 2.0 5.0))
    (set `CharacterMovementComponent.MaxWalkSpeed` 350.0 (`self.CharacterMovement`))
    (`|AIMoveTo` self (`NavigationSystemV1.K2_GetRandomReachablePointInRadius` _returnvalue 1000.0 null null) null)))

(event `self.StaticMesh.OnComponentHit`
  (params (HitComponent :type "PrimitiveComponent Object Reference") (OtherActor :type "Actor Object Reference") (OtherComp :type "PrimitiveComponent Object Reference") (NormalImpulse :type "Vector Structure") (Hit :type "HitResult Structure (by ref)")))

(event `self.Sphere1.OnComponentHit`
  (params (HitComponent :type "PrimitiveComponent Object Reference") (OtherActor :type "Actor Object Reference") (OtherComp :type "PrimitiveComponent Object Reference") (NormalImpulse :type "Vector Structure") (Hit :type "HitResult Structure (by ref)"))
  ;[1 1 1] Moo on overlap
)

(event `self.Sphere1.OnComponentBeginOverlap`
  (params (OverlappedComponent :type "PrimitiveComponent Object Reference") (OtherActor :type "Actor Object Reference") (OtherComp :type "PrimitiveComponent Object Reference") (OtherBodyIndex :type Integer) (bFromSweep :type Boolean) (SweepResult :type "HitResult Structure (by ref)"))
  ;[1 1 1] Moo on overlap
  (`/Engine/EditorBlueprintResources/StandardMacros.DoOnce` false :!label _label
    (:`Completed`
      (`GameplayStatics.PlaySoundAtLocation` "/Game/JEMO/JEMO_ASSETS/Sounds/cow-moo-wav_Cue.cow-moo-wav_Cue" (`SceneComponent.K2_GetComponentLocation` OverlappedComponent) (struct) 1.0 1.0 0.0 "/Game/Mixed_FREE_Template_Assets/MilitaryWeapSilver/Sound/Attenuation/WeaponShot_att.WeaponShot_att" null null)
      (`KismetSystemLibrary.Delay` 4.0)
      (goto _label :!via `Reset`))))

(fn `UserConstructionScript`)