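; Moon actor Blueprint with moon, glow and directional light components for a night sky.
; The construction script aims the actor's X axis from its location toward an Origin point and applies a uniform Scale.
; A DayToNight timeline would drive moon opacity, glow density and light intensity, but nothing plays it.
; The NightTransition and DayTransition events are empty stubs.
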(event `Night Transition`)

(event `Day Transition`)

(fn `UserConstructionScript`
  (bind _scale (`self.Scale`))
  (`self.K2_SetActorRotation` (`KismetMathLibrary.Conv_VectorToRotator` (`KismetMathLibrary.Normal` (- (`self.Origin`) (`self.K2_GetActorLocation`)))))
  (`self.SetActorScale3D` (`KismetMathLibrary.MakeVector` _scale _scale _scale)))